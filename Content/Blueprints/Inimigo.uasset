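; Enemy actor (Inimigo) that takes health changes and damages the player on contact.
; AlterarVida passes the delta to CalcularVIda and destroys the enemy once IsDead is set.
; On BeginPlay, a collision capsule moves to the mesh's "areadano" socket and attaches there to follow it as a hit area.
; Overlapping an actor tagged "player" that implements ISofrerDano sends it a fixed AlterarVida interface message.
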(event OnComponentBeginOverlap(CollisionCapsule)
  (params (OverlappedComponent :type Primitive%20Component%20Object%20Reference) (OtherActor :type Actor%20Object%20Reference) (OtherComp :type Primitive%20Component%20Object%20Reference) (OtherBodyIndex :type Integer) (bFromSweep :type Boolean) (SweepResult :type Hit%20Result%20Structure%20%28by%20ref%29))
  ;[1 1 1] Dano no player
  ;;[1 1 1] Comment
  (if (Utilities|DoesObjectImplementInterface OtherActor "/Game/Blueprints/ISofrerDano.ISofrerDano_C")
    (if (Actor|ActorHasTag OtherActor "player")
      (Class|ISofrerDano|AlterarVida(Message) OtherActor 2e+01))))

(event EventBeginPlay
  ;[1 1 1] Dano no player
  ;;[1 1 1] Para o socket segui o player
  (Transformation|SetWorldTransform (Variables|Default|GetCollision%20Capsule) (Transformation|GetSocketTransform (Variables|Character|GetMesh) "areadano" "RTS_World") false false)
  (Transformation|AttachComponentToComponent (Variables|Default|GetCollision%20Capsule) (Variables|Character|GetMesh) "areadano" "KeepWorld" "KeepWorld" "KeepWorld" true))

(event EventAlterarVida
  (params (Delata :type Float%20%28single-precision%29))
  ;[1 1 1] Calculando vida inimigo
  (CallFunction|CalcularVIda Delata)
  (if (Variables|Default|GetisDead)
    (Actor|DestroyActor)))

(fn ConstructionScript)