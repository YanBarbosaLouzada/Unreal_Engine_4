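; Enemy AI controller that switches its pawn between idle, chasing and attacking based on distance to the player.
; A looping one-second timer runs Seguir, which measures that distance and calls Atancando at close range, Andando at mid range or Parado beyond.
; Andando issues AI MoveTo toward the player, while the other two stop movement.
; Each state sets the Moveandando and Moveatacando flags; the attack state itself applies no damage.
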(event Custom|Parado
  ;[0.9177 0.2628 1] Parado
  (AI|Navigation|StopMovement)
  (Variables|Default|Setmoveandando false)
  (Variables|Default|Setmoveatacando false))

(event Custom|Atancando
  ;[1 0.1731 0.4366] Atancando
  (AI|Navigation|StopMovement)
  (Variables|Default|Setmoveandando false)
  (Variables|Default|Setmoveatacando true))

(event Custom|Andando
  ;[1 1 1] Andando
  (AI|AIMoveTo (Pawn|GetControlledPawn) "0, 0, 0" (Game|GetPlayerCharacter 0) 5.0 false
    (:then
      (Variables|Default|Setmoveandando true)
      (Variables|Default|Setmoveatacando false))))

(event Custom|Seguir
  ;[1 1 1] Pegardistancia
  (Variables|Default|SetDistancia (Transformation|GetDistanceTo (Pawn|GetControlledPawn) (Game|GetPlayerCharacter 0)))
  ;[1 1 1] Contoller inimigo
  (if (<= (Variables|Default|GetDistancia) 1.5e+02)
    (CallFunction|Atancando)
    (elif (<= (Variables|Default|GetDistancia) 7.5e+02)
      (CallFunction|Andando)
      (else
        (CallFunction|Parado)))))

(event EventBeginPlay
  (Utilities|Time|SetTimerbyFunctionName 0 "Seguir" 1.0 true))

(event EventTick
  (params (DeltaSeconds :type Float%20%28single-precision%29)))

(fn ConstructionScript)