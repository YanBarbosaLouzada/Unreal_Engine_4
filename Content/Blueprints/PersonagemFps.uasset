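; First-person player character Blueprint that handles movement, camera look, weapon use and death.
; Axis inputs drive movement relative to control rotation and camera yaw and inverted pitch.
; On BeginPlay it spawns an ArmaPersonagem weapon at the mesh's ArmaSocket and attaches it, then left mouse calls the weapon's Atirar to fire.
; AlterarVida passes health changes to CalcularVIda and destroys the actor when IsDead is set.
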(event EventBeginPlay
  (bind _mesh (Variables|Character|GetMesh))
  ;[1 1 1] Configurando Arma
  (bind _returnvalue (Game|SpawnActorfromClass "/Game/Blueprints/ArmaPersonagem.ArmaPersonagem_C" (Transformation|GetSocketTransform _mesh "ArmaSocket" "RTS_World") "Undefined" 0 0))
  (bind _output_get (Variables|Default|SetArma _returnvalue))
  (Transformation|AttachComponentToComponent _output_get _mesh "ArmaSocket" "KeepWorld" "KeepWorld" "KeepWorld" true))

(event EventAlterarVida
  (params (Delata :type Float%20%28single-precision%29))
  ;[1 1 1] Calculando vida do player
  (CallFunction|CalcularVIda Delata)
  (if (Variables|Default|GetisDead)
    (Actor|DestroyActor)))

(event Input|AxisEvents|InputAxisMoveForwards
  (params (AxisValue :type Float%20%28single-precision%29))
  ;[1 1 1] Aula1(Progamação)
  ;;[0.1524 0 1] Movimento do Player
  (Pawn|Input|AddMovementInput (Math|Vector|GetForwardVector (Pawn|GetControlRotation :!class /Script/Engine.Pawn)) AxisValue false))

(event Input|AxisEvents|InputAxisMoveRight
  (params (AxisValue :type Float%20%28single-precision%29))
  ;[1 1 1] Aula1(Progamação)
  ;;[0.1524 0 1] Movimento do Player
  (Pawn|Input|AddMovementInput (Math|Vector|GetRightVector (Pawn|GetControlRotation :!class /Script/Engine.Pawn)) AxisValue false))

(event Input|AxisEvents|InputAxisLookUP
  (params (AxisValue :type Float%20%28single-precision%29))
  ;[1 1 1] Aula1(Progamação)
  ;;[0.1331 0 1] Movimentação da Camera
  (Pawn|Input|AddControllerPitchInput (* AxisValue -1.0)))

(event Input|AxisEvents|InputAxisLookRight
  (params (AxisValue :type Float%20%28single-precision%29))
  ;[1 1 1] Aula1(Progamação)
  ;;[0.1331 0 1] Movimentação da Camera
  (Pawn|Input|AddControllerYawInput AxisValue))

(event Input|MouseEvents|LeftMouseButton
  (params (Key :type Key%20Structure :default "None"))
  ;[1 1 1] Usando Arma
  (:Pressed
    (bind _asarma_personagem (Utilities|Casting|CastToArmaPersonagem (Variables|Default|GetArma)))
    (Default|Atirar _asarma_personagem)))

(fn ConstructionScript)